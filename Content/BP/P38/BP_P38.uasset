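; P-38 aircraft that can fly along a spline track or be steered by player input, with gunfire on the Fire action.
; If FollowTrack is set, BeginPlay plays Running and starts a timeline that teleports the actor along the spline, scaled by FollowDuration and offset by FollowDelay.
; THR and ROLL axes directly set fuselage Y and X velocity; ROLL also prints a debug value.
; Gunsfire plays while Fire is held.
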(event Custom|Follow
  (Components|Timeline|SetPlayRate (Variables|Default|GetTimeline) (/ 1.0 (Variables|Default|GetFollowDuration)))
  (Components|Timeline|SetNewTime (Variables|Default|GetTimeline) (Variables|Default|GetFollowDelay))
  (bind _alpha (Timeline|Timeline Play)
    (:Update
      (bind _output_get (Variables|Default|SetAlpha _alpha))
      (Transformation|SetActorLocationAndRotation (Spline|GetLocationatDistanceAlongSpline (Variables|/Game/BP/Track.Track_C|GetPath (Variables|Components|GetTrack)) (* _output_get (Spline|GetSplineLength (Variables|/Game/BP/Track.Track_C|GetPath (Variables|Components|GetTrack)))) "World") (Spline|GetRotationatDistanceAlongSpline (Variables|/Game/BP/Track.Track_C|GetPath (Variables|Components|GetTrack)) (* _output_get (Spline|GetSplineLength (Variables|/Game/BP/Track.Track_C|GetPath (Variables|Components|GetTrack)))) "World") false true))))

(event EventBeginPlay
  (if (Variables|Default|GetFollowTrack)
    (CallFunction|Follow)
    (Audio|Components|Audio|Play (Variables|Default|Getrunning) 0.0)))

(event Input|ActionEvents|InputActionFire
  (params (Key :type Key%20Structure :default "None"))
  (bind _gunsfire (Variables|Default|Getgunsfire))
  (:Pressed
    (Audio|Components|Audio|Play _gunsfire 0.0))
  (:Released
    (Audio|Components|Audio|Stop _gunsfire)))

(event Input|AxisEvents|InputAxisTHR
  (params (AxisValue :type Float%20%28single-precision%29))
  (bind _returnvalue (Physics|GetPhysicsLinearVelocity (Variables|Default|GetSM_Fuselage) "None"))
  (Physics|SetPhysicsLinearVelocity (Variables|Default|GetSM_Fuselage) (Math|Vector|MakeVector (.x _returnvalue) (* AxisValue (Variables|Default|GetVerticalSpeedScale)) (.z _returnvalue)) false "None"))

(event Input|AxisEvents|InputAxisROLL
  (params (AxisValue :type Float%20%28single-precision%29))
  (bind _returnvalue (Physics|GetPhysicsLinearVelocity (Variables|Default|GetSM_Fuselage) "None"))
  (Physics|SetPhysicsLinearVelocity (Variables|Default|GetSM_Fuselage) (Math|Vector|MakeVector (* AxisValue (Variables|Default|GetHorizontalSpeedScale)) (.y _returnvalue) (.z _returnvalue)) false "None")
  (Development|PrintString (Utilities|String|Append "Rr=" (Utilities|String|ToString(Float) (* AxisValue (Variables|Default|GetRollRate))))))

(fn ConstructionScript)